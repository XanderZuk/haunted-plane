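; Monster character that flags when it sees the player, using a PawnSensing component.
; On seeing a BP_HorrorCharacter, it sets the HasSeenPlayer bool to true on its AI controller's Blackboard; this graph never clears it.
; It also carries horror-character touch input events that forward thumbsticks to move and aim, and the jump touch to sprint start and end.
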(event OnSeePawn(PawnSensing)
  (params (Pawn :type Pawn%20Object%20Reference))
  (Utilities|Casting|CastToBP_HorrorCharacter Pawn)
  (AI|Components|Blackboard|SetValueasBool (AI|GetBlackboard (AI|GetAIController self)) (Utilities|Name|MakeLiteralName "HasSeenPlayer") true))

(event EventPrimaryThumbstick
  (params (Axis :type Vector%202D%20Structure))
  ;[1 1 1] Touch Inputs for Horror Character
  (Class|HauntedPlaneCharacter|DoMove (.x Axis) (.y Axis)))

(event EventTouchJumpStart
  ;[1 1 1] Touch Inputs for Horror Character
  (Class|HorrorCharacter|DoStartSprint))

(event EventTouchJumpEnd
  ;[1 1 1] Touch Inputs for Horror Character
  (Class|HorrorCharacter|DoEndSprint))

(event EventSecondaryThumbstick
  (params (Axis :type Vector%202D%20Structure))
  ;[1 1 1] Touch Inputs for Horror Character
  (Class|HauntedPlaneCharacter|DoAim (.x Axis) (.y Axis)))

(fn ConstructionScript)