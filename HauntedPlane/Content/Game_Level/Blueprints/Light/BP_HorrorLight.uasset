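; BP_HorrorLight is a configurable light prop, pairing a SpotLight with a Cylinder mesh, with optional flicker.
; Its Construction Script sets the spotlight's color and a seeded random intensity, then copies both into the cylinder's Custom Primitive Data.
; UseLightFlicker selects the cylinder's flickering or plain material and applies the LF_Flicker light function to the spotlight, so no runtime Blueprint logic runs.
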(event EventBeginPlay)

(event Collision|EventActorBeginOverlap
  (params (OtherActor :type Actor%20Object%20Reference)))

(event EventTick
  (params (DeltaSeconds :type Float%20%28single-precision%29)))

(fn ConstructionScript
  (bind _use_light_flicker (Variables|Default|GetUse%20Light%20Flicker))
  (bind _new_light_color (Variables|Default|GetNew%20Light%20Color))
  (bind (_r _g _b _a) (Utilities|Struct|BreakLinearColor _new_light_color))
  (bind _output_get (Variables|Default|SetRandomIntensity (Math|Random|RandomFloatinRangefromStream (Variables|Default|GetSeed) 0.3 1.4)))
  (Rendering|Components|Light|SetIntensity (Variables|Default|GetSpotLight) _output_get)
  (Rendering|Components|Light|SetLightColor (Variables|Default|GetSpotLight) _new_light_color true)
  (Rendering|Material|SetDefaultCustomPrimitiveDataVector4 (Variables|Default|GetCylinder) 1 (Math|Vector4|MakeVector4 _r _g _b _a))
  (Rendering|Material|SetDefaultCustomPrimitiveDataFloat (Variables|Default|GetCylinder) 0 _output_get)
  (Rendering|Material|SetMaterial (Variables|Default|GetCylinder) 0 (select _use_light_flicker "/Game/Variant_Horror/Blueprints/Light/Assets/Materials/MI_FlickeringLight.MI_FlickeringLight" "/Game/Variant_Horror/Blueprints/Light/Assets/Materials/M_Light.M_Light"))
  (Rendering|Components|Light|SetLightFunctionMaterial (Variables|Default|GetSpotLight) (select _use_light_flicker "/Game/Variant_Horror/Blueprints/Light/Assets/Materials/LF_Flicker.LF_Flicker" 0)))