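; BP_MazeSpawner is a Blueprint that generates a maze at BeginPlay and builds its walls.
; It calls GenerateMap with map size, initial states, generation count and weights for complexity, solvability and openness, suggesting an evolutionary search defined outside these graphs.
; It walks the returned rows and adds a WallSegment instance for each cell equal to 1, placed on an X/Y grid spaced by Offset.
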(event EventBeginPlay
  (bind _offset (Variables|Default|GetOffset))
  (bind _returnvalue (Class|ProceduralGeneration|GenerateMap (Variables|Default|GetMapSize) (Variables|Default|GetInitialStates) (Variables|Default|GetGenerations) (Variables|Default|GetComplexityWeight) (Variables|Default|GetSolvabilityWeight) (Variables|Default|GetOpennessWeight)))
  (for (_array_element _array_index) _returnvalue
    (for (_array_element_2 _array_index_2) (Utilities|Struct|BreakMapRow _array_element)
      (if (== _array_element_2 1)
        (Components|InstancedStaticMesh|AddInstance (Variables|Default|GetWallSegment) (Math|Transform|MakeTransform (Math|Vector|MakeVector (* _array_index_2 _offset) (* _offset _array_index) 0.0) "0, 0, 0" "1.000000,1.000000,1.000000") false)))))

(fn ConstructionScript)