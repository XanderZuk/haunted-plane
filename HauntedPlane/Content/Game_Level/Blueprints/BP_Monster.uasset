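; BP_Monster is a monster character for a horror game that notifies its AI when it sees the player.
; Its PawnSensing component filters seen pawns to HorrorCharacter and sets the HasSeenPlayer blackboard key to true on the monster's AI controller.
; Nothing in this graph clears that key.
; It also carries First Person Character touch input handlers that forward to move, aim and jump functions.
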(event OnSeePawn(PawnSensing)
  (params (Pawn :type Pawn%20Object%20Reference))
  (Utilities|Casting|CastToHorrorCharacter Pawn)
  (AI|Components|Blackboard|SetValueasBool (AI|GetBlackboard (AI|GetAIController self)) (Utilities|Name|MakeLiteralName "HasSeenPlayer") true))

(event EventPrimaryThumbstick
  (params (Axis :type Vector%202D%20Structure))
  ;[1 1 1] Touch Inputs for First Person Character
  (Class|HauntedPlaneCharacter|DoMove (.x Axis) (.y Axis)))

(event EventTouchJumpStart
  ;[1 1 1] Touch Inputs for First Person Character
  (Class|HauntedPlaneCharacter|DoJumpStart))

(event EventTouchJumpEnd
  ;[1 1 1] Touch Inputs for First Person Character
  (Class|HauntedPlaneCharacter|DoJumpEnd))

(event EventSecondaryThumbstick
  (params (Axis :type Vector%202D%20Structure))
  ;[1 1 1] Touch Inputs for First Person Character
  (Class|HauntedPlaneCharacter|DoAim (.x Axis) (.y Axis)))

(fn ConstructionScript)